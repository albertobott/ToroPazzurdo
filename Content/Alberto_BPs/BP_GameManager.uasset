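; Game manager for a crash-style betting round with an exponentially rising value and a randomly chosen stop target.
; BeginPlay starts the round, creates two timer widgets without adding them to the viewport, and caches the PlayerSpot actor.
; ExponentialIncrement advances time on each call and returns formatted text, while Tick checks for exact equality with the target to store the floored score.
; Cash-out handling only zeroes the amount, and bet loss is an empty stub.
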(event Custom|StartGame
  ;[0.3672 0.653 1] Inizio Partita
  (Variables|Default|SetPlayerCashOut false)
  (Variables|Default|SetisGameRunning true)
  (Variables|Default|SetLastScore 0.0)
  (Variables|Default|SetRandomInt (Math|Random|RandomIntegerinRange 15 40))
  (if (<= (Math|Random|RandomInteger 100) 15)
    _))

(event EventBeginPlay
  (CallFunction|StartGame)
  (Utilities|FlowControl|Sequence
    (:then_0
      ;[1 1 1] Set Score
      (bind _returnvalue (UserInterface|CreateWidget "/Game/Luca_Folder/BP_Timer.BP_Timer_C" (Game|GetPlayerController 0)))
      (Variables|Default|SetWidget%20Timer _returnvalue))
    (:then_1
      (bind _returnvalue_2 (Actor|GetActorOfClass "/Game/Luca_Folder/PlayerSpot.PlayerSpot_C"))
      (Variables|Default|SetPlayerSpot _returnvalue_2))
    (:then_2
      (bind _returnvalue_3 (UserInterface|CreateWidget "/Game/Luca_Folder/BP_Timer.BP_Timer_C" (Game|GetPlayerController 0)))
      (Variables|Default|SetWidgetSaldo _returnvalue_3))))

(event EventTick
  (params (DeltaSeconds :type Float%20%28single-precision%29))
  (if (Variables|Default|GetisGameRunning)
    (if (== (* (Variables|Default|GetExponentialFloat) 1e+01) (Variables|Default|GetRandomInt))
      (Variables|Default|Settime 0.0)
      (Variables|Default|SetLastScore (Math|Conversions|ToFloat(Integer) (Math|Float|Floor (Variables|Default|GetExponentialFloat))))
      (Variables|Default|SetExponentialFloat 0.0)
      (Variables|Default|SetRandomInt 0))))

(fn ConstructionScript)

(fn ExponentialIncrement
  (if (Variables|Default|GetisGameRunning)
    (bind _output_get (Variables|Default|SetTime (+ (Utilities|Time|GetWorldDeltaSeconds) (Variables|Default|Gettime))))
    (bind _output_get_2 (Variables|Default|SetExponentialFloat (- (Math|Float|Power 1.1 (Math|Float|Clamp(Float) _output_get 1.0 1e+03)) 0.1)))
    (return (Utilities|Text|ToText(Float) _output_get_2 "HalfToEven" false true 1 324 2 2))
    (else
      (return (Utilities|Text|ToText(Float) (Variables|Default|GetLastScore) "HalfToEven" false true 1 324 2 2)))))

(fn SaveCashOutScore
  (params (Score :type Float%20%28double-precision%29))
  (Variables|Default|SetCashOutAmount 0.0))

(fn BetLoss)