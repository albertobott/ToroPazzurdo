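; Game manager for a crash-style betting game, running rounds where an exponentially growing multiplier climbs until a random drop.
; A looping timer rolls two random numbers within time-dependent ranges, and Tick ends the round when they match, saving the last score.
; BetTime pauses before restarting, and a small chance skips straight to it as an instant drop.
; It also creates timer and balance widgets, while cash-out and loss functions are stubs.
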(event Custom|TestDelta
  ;[1 1 1] Logica game
  (bind _output_get (Variables|Default|SetTimerRandNum (+ (Variables|Default|GetCheckAlSec) (Variables|Default|GetTimerRandNum))))
  (switch int (Math|Float|Floor (Math|Conversions|ToFloat(Integer) (/ _output_get 5)))
    (:Default
      (Variables|Default|SetRandomNum (Math|Random|RandomIntegerinRange 1 15))
      (Variables|Default|SetKeyNum (Math|Random|RandomIntegerinRange 1 15)))
    (:0
      (Variables|Default|SetRandomNum (Math|Random|RandomIntegerinRange 1 12))
      (Variables|Default|SetKeyNum (Math|Random|RandomIntegerinRange 1 12)))
    (:1
      (Variables|Default|SetRandomNum (Math|Random|RandomIntegerinRange 1 14))
      (Variables|Default|SetKeyNum (Math|Random|RandomIntegerinRange 1 14)))
    (:2
      (Variables|Default|SetRandomNum (Math|Random|RandomIntegerinRange 1 15))
      (Variables|Default|SetKeyNum (Math|Random|RandomIntegerinRange 1 15)))
    (:3
      (Variables|Default|SetRandomNum (Math|Random|RandomIntegerinRange 1 18))
      (Variables|Default|SetKeyNum (Math|Random|RandomIntegerinRange 1 18)))
    (:4
      (Variables|Default|SetRandomNum (Math|Random|RandomIntegerinRange 1 19))
      (Variables|Default|SetKeyNum (Math|Random|RandomIntegerinRange 1 19)))
    (:5
      (Variables|Default|SetRandomNum (Math|Random|RandomIntegerinRange 1 19))
      (Variables|Default|SetKeyNum (Math|Random|RandomIntegerinRange 1 19)))
    (:6
      (Variables|Default|SetRandomNum (Math|Random|RandomIntegerinRange 1 19))
      (Variables|Default|SetKeyNum (Math|Random|RandomIntegerinRange 1 19)))
    (:7
      (Variables|Default|SetRandomNum (Math|Random|RandomIntegerinRange 1 18))
      (Variables|Default|SetKeyNum (Math|Random|RandomIntegerinRange 1 18)))
    (:8
      (Variables|Default|SetRandomNum (Math|Random|RandomIntegerinRange 1 17))
      (Variables|Default|SetKeyNum (Math|Random|RandomIntegerinRange 1 17)))
    (:9
      (Variables|Default|SetRandomNum (Math|Random|RandomIntegerinRange 1 14))
      (Variables|Default|SetKeyNum (Math|Random|RandomIntegerinRange 1 14)))
    (:10
      (Variables|Default|SetRandomNum (Math|Random|RandomIntegerinRange 1 11))
      (Variables|Default|SetKeyNum (Math|Random|RandomIntegerinRange 1 11)))))

(event Custom|Test1
  ;[1 1 1] Logica game
  (bind _returnvalue (Utilities|Time|SetTimerbyEvent (delegate Custom|TestDelta) (Variables|Default|GetCheckAlSec) true))
  (Variables|Default|SetNewVar_0 _returnvalue))

(event Custom|StartGame
  ;[0.3672 0.653 1] Inizio Partita
  (Variables|Default|SetPlayerCashOut false)
  (Variables|Default|SetisGameRunning true)
  (Variables|Default|SetLastScore 0.0)
  (if (<= (Math|Random|RandomInteger 100) 5)
    (CallFunction|BetTime)
    (Development|PrintString "Drop Istantaneo")
    (else
      (CallFunction|Test1))))

(event Custom|BetTime
  ;[1 0.9826 0.4479] Intervallo di 10 sec a partita
  (Variables|Default|SetisGameRunning false)
  (Variables|Default|SetIsGameEnd true)
  (Development|PrintString "Timer 5 sec" true true "(R=0.000000,G=0.660000,B=1.000000,A=1.000000)" 5.0)
  (Utilities|FlowControl|Delay 5.0)
  (CallFunction|StartGame))

(event EventBeginPlay
  (CallFunction|StartGame)
  (Utilities|FlowControl|Sequence
    (:then_0
      ;[1 1 1] Set Score
      (bind _returnvalue (UserInterface|CreateWidget "/Game/Alberto_Folder/BP_Timer.BP_Timer_C" (Game|GetPlayerController 0)))
      (bind _output_get (Variables|Default|SetWidget%20Timer _returnvalue))
      (UserInterface|Viewport|AddtoViewport _output_get 0))
    (:then_1
      (bind _returnvalue_2 (Actor|GetActorOfClass "/Game/Luca_Folder/PlayerSpot.PlayerSpot_C"))
      (Variables|Default|SetPlayerSpot _returnvalue_2))
    (:then_2
      (bind _returnvalue_3 (UserInterface|CreateWidget "/Game/Alberto_Folder/W_Saldo.W_Saldo_C" (Game|GetPlayerController 0)))
      (bind _output_get_2 (Variables|Default|SetWidgetSaldo _returnvalue_3))
      (UserInterface|Viewport|AddtoViewport _output_get_2 0))))

(event EventTick
  (params (DeltaSeconds :type Float%20%28single-precision%29))
  (if (Variables|Default|GetisGameRunning)
    (Development|PrintString (Utilities|String|ToString(Integer) (Variables|Default|GetRandomNum)) true true "(R=1.000000,G=0.949367,B=0.000000,A=1.000000)")
    (Development|PrintString (Utilities|String|ToString(Integer) (Variables|Default|GetKeyNum)))
    (if (== (Variables|Default|GetRandomNum) (Variables|Default|GetKeyNum))
      (Development|PrintString "Dropped")
      (Utilities|Time|ClearandInvalidateTimerbyHandle (Variables|Default|GetNewVar_0))
      (Variables|Default|SetTimerRandNum 0.0)
      (Variables|Default|Settime 0.0)
      (bind _output_get (Variables|Default|SetLastScore (Variables|Default|GetExponentialFloat)))
      (Variables|Default|SetExponentialFloat 0.0)
      (Development|PrintString (Utilities|String|ToString(Float) _output_get) true true "(R=0.233631,G=1.000000,B=0.000000,A=1.000000)")
      (Utilities|FlowControl|Sequence
        (:then_0
          (CallFunction|BetTime)
          (Variables|Default|SetKeyNum 1)
          (Variables|Default|SetRandomNum 0))))))

(fn ConstructionScript)

(fn ExponentialIncrement
  (if (Variables|Default|GetisGameRunning)
    (bind _output_get (Variables|Default|SetTime (+ (Utilities|Time|GetWorldDeltaSeconds) (Variables|Default|Gettime))))
    (bind _output_get_2 (Variables|Default|SetExponentialFloat (- (Math|Float|Power 1.1 (Math|Float|Clamp(Float) _output_get 1.0 1e+03)) 0.1)))
    (return (Utilities|Text|ToText(Float) _output_get_2 "HalfToEven" false true 1 324 2 2))
    (else
      (return (Utilities|Text|ToText(Float) (Variables|Default|GetLastScore) "HalfToEven" false true 1 324 2 2)))))

(fn SaveCashOutScore
  (params (Score :type Float%20%28double-precision%29))
  (Variables|Default|SetCashOutAmount 0.0))

(fn BetLoss)